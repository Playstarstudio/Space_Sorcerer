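; BP_NarrativeObject is an interactable main menu object that drives the intro narrative widget.
; On BeginPlay it creates WBP_Intro, adds it to the viewport, flags it visible, starts looping music through BotFight_GameInstance and prints a debug string.
; Interact calls Continue on the widget and increments its IntroTableIndex, or runs the same creation path if the Visible flag is unset.
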(event `/Game/MainMenu/BPI_Interact.Interact`
  (if (`self.Visible`)
    (`self.ContinueNarrative`)
    (else
      (`self.InstantiateWidget`))))

(event `InstantiateWidget`
  (bind _returnvalue (`|CreateWidget` "/Game/MainMenu/WBP_Intro.WBP_Intro_C" :!label _label))
  (bind _output_get (set `self.UIWidget` _returnvalue))
  (`UserWidget.AddToViewport` _output_get 0)
  (set `self.Visible` true)
  (bind _asbot_fight_game_instance (cast `/Game/AI/AIBehaviors/BT_Assets/BotFight_GameInstance` (`GameplayStatics.GetGameInstance`)))
  (`/Game/AI/AIBehaviors/BT_Assets/BotFight_GameInstance.PlayMusic` _asbot_fight_game_instance "/Game/Audio/Music/MSS_MusicLoop.MSS_MusicLoop")
  (`KismetSystemLibrary.PrintString` "press6" true true (struct :`G` 1.0 :`B` 0.025927 :`A` 1.0)))

(event `self.ReceiveBeginPlay`
  (goto _label))

(event `ContinueNarrative`
  (bind _uiwidget (`self.UIWidget`))
  (`/Game/MainMenu/WBP_Intro.Continue` _uiwidget)
  (`/Engine/EditorBlueprintResources/StandardMacros.IncrementInt` (`/Game/MainMenu/WBP_Intro.Intro Table  Index` _uiwidget)))

(fn `UserConstructionScript`)