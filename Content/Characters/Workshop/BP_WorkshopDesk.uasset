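; Workshop desk that displays a rerollable selection of random items on its skeletal mesh and shows a key prompt when the wizard character overlaps it.
; BeginPlay fills the common item pool, then calls SpawnItems, which starts the Reroll montage and replaces each referenced item without waiting for it to finish.
; Slot index sets rarity (three common, one uncommon, one rare), and each new item snaps to its socket.
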(event `self.ReceiveBeginPlay`
  (bind _common_item_variants (`self.Common_Item_Variants`))
  (`KismetArrayLibrary.Array_Set` _common_item_variants 0 "/Game/AutoBattlerShop/Items/LaserGunItem.LaserGunItem_C")
  (`KismetArrayLibrary.Array_Set` _common_item_variants 1 "/Game/AutoBattlerShop/Items/CannonItem.CannonItem_C")
  (`KismetArrayLibrary.Array_Set` _common_item_variants 2 "/Game/AutoBattlerShop/Items/MaceItem.MaceItem_C")
  (`KismetArrayLibrary.Array_Set` _common_item_variants 3 "/Game/AutoBattlerShop/Items/KnightHelmet.KnightHelmet_C")
  (`KismetArrayLibrary.Array_Set` _common_item_variants 4 "/Game/AutoBattlerShop/Items/SpaceHelmet.SpaceHelmet_C")
  (`self.Spawn Items`))

(event `self.Interactive Box.OnComponentBeginOverlap`
  (params (OverlappedComponent :type "PrimitiveComponent Object Reference") (OtherActor :type "Actor Object Reference") (OtherComp :type "PrimitiveComponent Object Reference") (OtherBodyIndex :type Integer) (bFromSweep :type Boolean) (SweepResult :type "HitResult Structure (by ref)"))
  (cast `/Game/AutoBattlerShop/BP_WizardCharacter` OtherActor)
  (`KismetSystemLibrary.PrintString` "Press \"E\" to bring out the mouse!"))

(event `Spawn Items`
  (`|PlayMontage` (`self.SkeletalMesh`) "/Game/Characters/Workshop/Reroll.Reroll"
    (:`then`
      (for (_array_element _array_index) (`self.Item References`)
        (`self.K2_DestroyActor` _array_element)
        (switch `int` _array_index
          (:`0`
            (bind _output (`|GetArrayItem` (`self.Sockets`) _array_index))
            (bind _returnvalue (`SceneComponent.GetSocketTransform` (`self.SkeletalMesh`) _output "RTS_World"))
            (bind _returnvalue_2 (`|SpawnActorFromClass` (`KismetArrayLibrary.Array_Random` (`self.Common_Item_Variants`)) _returnvalue "Undefined" "MultiplyWithRoot" null null :!label _label))
            (set `self.NewItem` _returnvalue_2))
          (:`1`
            (goto _label))
          (:`2`
            (goto _label))
          (:`3`
            (bind _returnvalue_3 (`|SpawnActorFromClass` (`KismetArrayLibrary.Array_Random` (`self.Uncommon_Item_Variants`)) _returnvalue "Undefined" "MultiplyWithRoot" null null))
            (set `self.NewItem` _returnvalue_3))
          (:`4`
            (bind _returnvalue_4 (`|SpawnActorFromClass` (`KismetArrayLibrary.Array_Random` (`self.Rare_Item_Variants`)) _returnvalue "Undefined" "MultiplyWithRoot" null null))
            (bind _output_get (set `self.NewItem` _returnvalue_4))))
        (`KismetArrayLibrary.Array_Set` (`self.Item References`) _array_index _output_get)
        (`self.K2_AttachToComponent` (`self.NewItem`) (`self.SkeletalMesh`) _output "SnapToTarget" "SnapToTarget" "SnapToTarget" true)))))

(fn `UserConstructionScript`)