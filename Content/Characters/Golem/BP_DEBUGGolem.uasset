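; BP_DEBUGGolem is a debug golem character that assembles itself from debug parts at spawn.
; On BeginPlay it links itself to its AIC_ThirdPersonCharacter AI controller, then adds DebugPart and enables the Left and Right regions.
; After a short delay it gets the game instance and alerts it of the golem.
; The PartDataMod_Add region switch is empty, and a team/perception ID debug print is disconnected.
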(event `self.ReceiveBeginPlay`
  (bind _asaic_third_person_character (cast `/Game/AI/AIBehaviors/AIC_ThirdPersonCharacter` (`self.GetController`)))
  (bind _output_get (set `self.AIControllerReference` _asaic_third_person_character))
  (`/Game/AI/AIBehaviors/AIC_ThirdPersonCharacter.SetAssociatedGolem` _output_get self)
  (`self.AddPart` (`self.DebugPart`) (`self.Region`))
  (`self.SetRegion` "PR_Left" true)
  (`self.AddPart` (`self.DebugPart`) "PR_Right")
  (`self.SetRegion` "PR_Right" true)
  (`KismetSystemLibrary.Delay` 0.2)
  (`self.GetGameInstanceREF`)
  (`self.AlertGameInstanceOfGolem`))

(event `PartDataMod_Add`
  (switch `UGolemPartRegion` (`self.Region`)))

(fn `UserConstructionScript`
  (`parent.UserConstructionScript`))