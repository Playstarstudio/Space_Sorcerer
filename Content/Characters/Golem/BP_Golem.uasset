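; BP_Golem is an AI-controlled, team-based fighting robot assembled from attachable parts, registered with the BotFight game instance.
; AddPart mounts parts by region, feeding weapon ranges to the AI controller, while heads scale health and set ranged preference.
; Tick caches cannon cooldowns and movement angle toward the blackboard target location.
; Enemy hits retarget the golem and apply modified damage to its health bar, with death clearing targets and unregistering it.
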(event `PowerOff`
  (set `self.GolemEnabled` false))

(event `PowerOn`
  (set `self.GolemEnabled` true)
  (`self.PlayAnimMontage` "/Game/Characters/Golem/Animation/Animations/FullBones/DONOTUSE_Montages/Robo_Powerup.Robo_Powerup"))

(event `GetGameInstanceREF`
  (bind _asbot_fight_game_instance (cast `/Game/AI/AIBehaviors/BT_Assets/BotFight_GameInstance` (`GameplayStatics.GetGameInstance`)))
  (set `self.Game Instance Ref` _asbot_fight_game_instance))

(event `AlertGameInstanceOfGolem`
  (`/Game/AI/AIBehaviors/BT_Assets/BotFight_GameInstance.AddGolem` (`self.Game Instance Ref`) self))

(event `self.ReceiveTick`
  (params (DeltaSeconds :type "Float (single-precision)"))
  (if (not (`self.Dead`))
    (`self.HealthIncrementCheck`)
    (if (!= (`self.distanceToTarget`) -1.0)
      (`self.UpdateCannonData`)
      (`self.DetermineAngleVsMovement`))))

(event `ResetTargetEvent_Event`
  (`self.ResetTarget`))

(event `OnHealthChangeEvent_Event`
  (params (NewParam :type Integer))
  (`/Game/AI/AIBehaviors/AIC_ThirdPersonCharacter.UpdateHealthKey` (cast `/Game/AI/AIBehaviors/AIC_ThirdPersonCharacter` (`self.GetController`) :!pure true) NewParam))

(event `self.ReceivePossessed`
  (params (NewController :type "Controller Object Reference"))
  (`/Game/AI/AIBehaviors/AIC_ThirdPersonCharacter.UpdateHealthKey` (cast `/Game/AI/AIBehaviors/AIC_ThirdPersonCharacter` (`self.GetController`) :!pure true) (`self.CurrentHealth`)))

(event `self.ReceiveBeginPlay`
  (`self.UpdateHealthBar` (`KismetMathLibrary.Conv_IntToDouble` (`self.CurrentHealth`)))
  (bind _asaic_third_person_character (cast `/Game/AI/AIBehaviors/AIC_ThirdPersonCharacter` (`self.GetController`)))
  (bind _output_get (set `self.AIControllerReference` _asaic_third_person_character))
  (`/Game/AI/AIBehaviors/AIC_ThirdPersonCharacter.SetAssociatedGolem` _output_get self)
  (`KismetSystemLibrary.Delay` 0.2)
  (`self.GetGameInstanceREF`)
  (if (`self.InShop`)
    (set `self.TeamTracker` -1))
  (`self.AlertGameInstanceOfGolem`))

(fn `AddHeadValues`
  (params (NewHead :type "GolemHead Object Reference"))
  (bind _hpmod (`GolemHead.HpMod` NewHead))
  (set `self.preferRanged` (`GolemHead.PreferRanged` NewHead))
  (bind _output_get (set `self.CurrentHealth` (`KismetMathLibrary.FTrunc` (* (`self.CurrentHealth`) _hpmod))))
  (set `self.MaxHealth` (`KismetMathLibrary.FTrunc` (* _hpmod (`self.MaxHealth`))))
  (`self.OnHealthChangeEvent_Event` _output_get))

(fn `AddPart`
  (params (PartPrefab :type "Part Class Reference") (Region :type "UGolemPartRegion Enum" :default "PR_None"))
  (locals (NewPart :type "Part Object Reference") (NewRegion :type "UGolemPartRegion Enum"))
  (bind _newpart (`local.NewPart`))
  (bind _newpart_2 (`local.NewPart`))
  (bind _newpart_3 (`local.NewPart`))
  (if (`|EnumEquality` Region "PR_Head")
    (`self.RemoveHeadValues`))
  (bind _returnvalue (`self.AddCannon` PartPrefab Region (1.0 1.0 1.0)))
  (set `local.NewPart` _returnvalue)
  (switch `UGolemPartRegion` Region
    (:`PR_Left`
      (bind _returnvalue_2 (`self.PartAtLocation` "PR_Left"))
      (`self.SetRanges` _returnvalue_2 (`self.WeaponRangeMin_L`) (`self.WeaponRangeMax_L`))
      (`self.K2_SetActorRelativeRotation` _newpart_3 (`Part.partRotation` _newpart_3) false false :!label _label))
    (:`PR_Right`
      (bind _returnvalue_3 (`self.PartAtLocation` "PR_Left"))
      (`self.SetRanges` _returnvalue_3 (`self.WeaponRangeMin_R`) (`self.WeaponRangeMax_R`))
      (`self.K2_SetActorRelativeRotation` _newpart (`KismetMathLibrary.MakeRotator` (.roll (`Part.partRotation` _newpart)) (* (.pitch (`Part.partRotation` _newpart)) -1.0) (.yaw (`Part.partRotation` _newpart))) false false))
    (:`PR_Both_Hands`
      (goto _label))
    (:`PR_Head`
      (goto _label)))
  (`self.SetActorScale3D` _newpart_2 (* (`self.GetActorScale3D` _newpart_2) (`Part.partScaling` _newpart_2)))
  (`/Game/AI/AIBehaviors/AIC_ThirdPersonCharacter.UpdateRangeKeys` (`self.AIControllerReference`))
  (bind _asgolem_head (cast `GolemHead` (`local.NewPart`)))
  (`self.AddHeadValues` _asgolem_head))

(fn `DetermineAngleVsMovement`
  (bind _output_get (set `self.NormalizedMovementVector` (`KismetMathLibrary.Normal` (- (`BlackboardComponent.GetValueAsVector` (`AIBlueprintHelperLibrary.GetBlackboard` null) "Current_TargetLocation") (`self.K2_GetActorLocation`)))))
  (bind _output_get_2 (set `self.NormalizedForwardVector` (`self.GetActorForwardVector`)))
  (bind _returnvalue (`KismetMathLibrary.Dot_VectorVector` _output_get_2 _output_get))
  (bind _returnvalue_2 (`KismetMathLibrary.DegAcos` _returnvalue))
  (bind _output_get_3 (set `self.MovementAngle` (`KismetMathLibrary.SelectFloat` _returnvalue_2 (* _returnvalue_2 -1.0) (< _returnvalue 0.0)))))

(fn `Die`
  (params (Object :type "Object Object Reference") (Instigator :type "/Game/Characters/Golem/BP_Golem Object Reference"))
  (locals (NeutralPerc :type "GenericTeamId Structure"))
  (bind _capsulecomponent (`self.CapsuleComponent`))
  (bind _asbp_golem (cast `/Game/Characters/Golem/BP_Golem` Object))
  (`self.ResetTarget` _asbp_golem)
  (`/Game/AI/AIBehaviors/AIC_ThirdPersonCharacter.ResetTargetActorKey` (`/Game/Characters/Golem/BP_Golem.AIControllerReference` _asbp_golem))
  (set `self.Dead` true)
  (`MovementComponent.StopMovementImmediately` (`self.CharacterMovement`))
  (`self.DetachFromControllerPendingDestroy`)
  (`PrimitiveComponent.SetCollisionEnabled` _capsulecomponent "NoCollision")
  (`PrimitiveComponent.SetCollisionResponseToAllChannels` _capsulecomponent "ECR_Ignore")
  (`self.RemoveSelfFromInstigator` Instigator)
  (`/Game/AI/AIBehaviors/BT_Assets/BotFight_GameInstance.RemoveGolem` (`self.Game Instance Ref`) (`self.AIControllerReference`)))

(fn `HealthIncrementCheck`
  (if true
    _))

(fn `IsDistanceValid`
  (params (`Cannon Data` :type "Cannon Object Reference"))
  (returns (ReturnValue :type Boolean))
  (bind _distancetotarget (`self.distanceToTarget`))
  (return (and (<= _distancetotarget (`Cannon.MaxRange` `Cannon Data`)) (>= _distancetotarget (`Cannon.MinRange` `Cannon Data`)))))

(fn `ModifyDamageValues`
  (params (OtherGolem :type "/Game/Characters/Golem/BP_Golem Object Reference") (OriginalQuantity :type Integer))
  (returns (NewQuantity :type Integer))
  (locals (ReturnQuantity :type "Float (double-precision)"))
  (set `local.ReturnQuantity` (`KismetMathLibrary.Conv_IntToDouble` OriginalQuantity))
  (bind _returnvalue (`self.PartAtLocation` "PR_None"))
  (bind _asgolem_head (cast `GolemHead` _returnvalue)
    (:`then`
      (set `local.ReturnQuantity` (* (`GolemHead.RangeDamageMod` _asgolem_head) (`local.ReturnQuantity`))))
    (:`CastFailed`
      _))
  (bind _returnvalue_2 (`self.PartAtLocation` "PR_None"))
  (bind _asgolem_head_2 (cast `GolemHead` _returnvalue_2)
    (:`then`
      (set `local.ReturnQuantity` (/ (`local.ReturnQuantity`) (`GolemHead.DefenseMod` _asgolem_head_2))))
    (:`CastFailed`
      _))
  (return (`KismetMathLibrary.FTrunc` (`local.ReturnQuantity`))))

(fn `ReceiveDamage`
  (params (DamangeQuantity :type Integer) (Type :type "GolemDamageType Enum" :default "DT_Instant") (AdditionalInfo :type Integer) (Instigator :type "Object Object Reference"))
  (locals (NeutralPerc :type "GenericTeamId Structure") (InstigatorRef :type "Object Object Reference"))
  (bind _asbp_golem (cast `/Game/Characters/Golem/BP_Golem` Instigator :!pure true))
  (bind _returnvalue (- (`self.CurrentHealth`) (`self.ModifyDamageValues` _asbp_golem DamangeQuantity)))
  (set `local.InstigatorRef` Instigator)
  (`self.SetTarget` _asbp_golem)
  (if (!= (`Golem.TeamTracker` _asbp_golem) (`self.TeamTracker`))
    (if (`|EnumEquality` Type "DT_Instant")
      ; Weapon Impact SFX
      (`GameplayStatics.PlaySoundAtLocation` (`BlueprintMapLibrary.Map_Find` (`self.WeaponSFX`) AdditionalInfo) (`self.K2_GetActorLocation` _asbp_golem) (struct) 1.0 1.0 0.0 null null null null)
      (bind _output_get (set `self.CurrentHealth` _returnvalue))
      (`self.UpdateHealthBar` (`KismetMathLibrary.Conv_IntToDouble` _returnvalue))
      ; Send to Instigatorcannon then to instigatorgolem to reset targets
      (if (<= _output_get 0)
        (`self.Die` (`local.InstigatorRef`))))))

(fn `RemoveHeadValues`
  (bind _returnvalue (`self.PartAtLocation` "PR_Head"))
  (`/Engine/EditorBlueprintResources/StandardMacros.IsValid` _returnvalue
    (:`Is Valid`
      (bind _asgolem_head (cast `GolemHead` _returnvalue))
      (bind _hpmod (`GolemHead.HpMod` _asgolem_head))
      (bind _output_get (set `self.CurrentHealth` (`KismetMathLibrary.FTrunc` (/ (`self.CurrentHealth`) _hpmod))))
      (set `self.MaxHealth` (`KismetMathLibrary.FTrunc` (/ (`self.MaxHealth`) _hpmod)))
      (`self.OnHealthChangeEvent_Event` _output_get))))

(fn `RemoveSelfFromInstigator`
  (params (Instigator :type "/Game/Characters/Golem/BP_Golem Object Reference"))
  (`self.ResetTarget` Instigator))

(fn `SetRanges`
  (params (Part :type "Part Object Reference") (MinRange :type "Integer (by ref)") (MaxRange :type "Integer (by ref)"))
  (`|VariableSetRef` MinRange (`KismetMathLibrary.FTrunc` (`Part.MinRange` Part)))
  (`|VariableSetRef` MaxRange (`KismetMathLibrary.FTrunc` (`Part.MaxRange` Part))))

(fn `UpdateCannonData`
  (bind _returnvalue (`self.PartAtLocation` "PR_Left"))
  (if (`KismetSystemLibrary.IsValid` _returnvalue)
    (set `self.L_Cooldown` (`Part.CurrentCooldown` _returnvalue)))
  (bind _returnvalue_2 (`self.PartAtLocation` "PR_Right"))
  (if (`KismetSystemLibrary.IsValid` _returnvalue_2)
    (set `self.R_Cooldown` (`Part.CurrentCooldown` _returnvalue_2))))

(fn `UpdateHealthBar`
  (params (NewParam :type "Float (double-precision)"))
  (bind _returnvalue (`KismetMathLibrary.SafeDivide` (`KismetMathLibrary.Conv_IntToDouble` (`self.CurrentHealth`)) (`KismetMathLibrary.Conv_IntToDouble` (`self.MaxHealth`))))
  (bind _aswb_health_bar (cast `/Game/Characters/HealthBar/WB_HealthBar` (`WidgetComponent.GetUserWidgetObject` (`self.HeatlhBar`))))
  (bind _healthbar (`/Game/Characters/HealthBar/WB_HealthBar.Healthbar` _aswb_health_bar))
  (`ProgressBar.SetPercent` _healthbar _returnvalue)
  (if (or (== _returnvalue 1.0) (<= _returnvalue 0.0))
    (set `Widget.Visibility` "Hidden" _healthbar)
    (else
      (set `Widget.Visibility` "Visible" _healthbar)))
  (return))

(fn `UserConstructionScript`)