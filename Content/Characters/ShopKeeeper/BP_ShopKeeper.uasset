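; BP_ShopKeeper is a shop keeper actor meant to stock animal items, though its spawning logic is unfinished.
; On BeginPlay it fills the Items array with Badger, Fox, Rabbit and two Squirrel entries, then calls SpawnItems.
; SpawnItems is empty, so nothing spawns.
; A disconnected loop would spawn each class to the actor's right at a random forward or backward offset.
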(event `self.ReceiveBeginPlay`
  (bind _items (`self.Items`))
  (`KismetArrayLibrary.Array_Set` _items 0 "/Game/AutoBattlerShop/Items/Badger.Badger_C")
  (`KismetArrayLibrary.Array_Set` _items 1 "/Game/AutoBattlerShop/Items/Fox.Fox_C")
  (`KismetArrayLibrary.Array_Set` _items 2 "/Game/AutoBattlerShop/Items/Rabbit.Rabbit_C")
  (`KismetArrayLibrary.Array_Set` _items 3 "/Game/AutoBattlerShop/Items/Squirrel.Squirrel_C")
  (`KismetArrayLibrary.Array_Set` _items 4 "/Game/AutoBattlerShop/Items/Squirrel.Squirrel_C")
  (`self.Spawn Items`))

(event `Key|Seven`
  (params (Key :type "Key Structure")))

(event `Key|SpaceBar`
  (params (Key :type "Key Structure")))

(event `Spawn Items`)

(fn `UserConstructionScript`)