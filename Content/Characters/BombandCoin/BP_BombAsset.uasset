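; BP_BombAsset is a bomb actor that bobs up and down while spinning in place.
; Each Tick offsets the static mesh vertically along a sine wave of game time and yaws the whole actor by a fixed step.
; Both motions apply per frame without delta-time scaling, so they depend on frame rate.
; BeginPlay caches the actor's starting location, which this graph never reads, and no overlap or explosion logic is present.
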(event `self.ReceiveBeginPlay`
  (set `self.BaseLocation` (`self.K2_GetActorLocation` self)))

(event `self.ReceiveTick`
  (params (DeltaSeconds :type "Float (single-precision)"))
  (`SceneComponent.K2_AddWorldOffset` (`self.StaticMesh`) (`KismetMathLibrary.MakeVector` 0.0 0.0 (* (* (`KismetMathLibrary.DegSin` (* (`KismetSystemLibrary.GetGameTimeInSeconds`) 250.0)) 0.01111) 60.0)) false false)
  (`self.K2_AddActorLocalRotation` (`KismetMathLibrary.MakeRotator` 0.0 0.0 -3.0)))

(fn `UserConstructionScript`)