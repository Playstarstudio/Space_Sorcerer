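; BP_PatrolPoint is a placeable actor that registers itself as a search point for the AI when the game begins.
; After a short delay on BeginPlay, it casts the game instance to BotFight_GameInstance and stores the reference.
; It then passes itself to the game instance's AddSearchPoint, which adds it to an array of search points.
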(event `self.ReceiveBeginPlay`
  (`KismetSystemLibrary.Delay` 0.1)
  (`self.GetGameInstanceREF`)
  (`self.AlertGameInstance`))

(event `GetGameInstanceREF`
  ; Get a reference to the game instance
  (bind _asbot_fight_game_instance (cast `/Game/AITestEntity/AIBehaviors/BT_Assets/BotFight_GameInstance` (`GameplayStatics.GetGameInstance`)))
  (set `self.GameInstanceREF` _asbot_fight_game_instance))

(event `AlertGameInstance`
  ; At Beginning of Game, Add to array of search points
  (`/Game/AITestEntity/AIBehaviors/BT_Assets/BotFight_GameInstance.AddSearchPoint` (`self.GameInstanceREF`) self))

(fn `UserConstructionScript`)