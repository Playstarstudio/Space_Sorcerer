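; BP_Cannon is a cannon actor, under TestingObjects, that launches a physics-driven projectile when its Fire event is called.
; FireProjectile spawns a BulletInGame at the cannon, moves it ahead along the Cube's forward vector, then applies an AddedForce-scaled impulse to its Sphere.
; Cooldown logic is left unwired: the Fire check compares constants and always passes, and Tick does nothing.
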(event `self.Fire`
  (if (<= 0.0 0.0)
    (`self.FireProjectile`)))

(event `self.ReceiveTick`
  (params (DeltaSeconds :type "Float (single-precision)")))

(fn `FireProjectile`
  (bind _returnvalue (`|SpawnActorFromClass` "/Game/TestingObjects/BulletInGame.BulletInGame_C" (`KismetMathLibrary.MakeTransform` (`self.K2_GetActorLocation`) (`self.K2_GetActorRotation`)) "Undefined" "MultiplyWithRoot" null (`self.GetInstigator`)))
  (`self.K2_SetActorLocation` _returnvalue (+ (`self.K2_GetActorLocation`) (* (`SceneComponent.GetForwardVector` (`self.Cube`)) (50.0 50.0 50.0))) false false)
  (`PrimitiveComponent.AddImpulse` (`/Game/TestingObjects/BulletInGame.Sphere` _returnvalue) (* (`SceneComponent.GetForwardVector` (`self.Cube`)) (`self.AddedForce`)) "None" false))

(fn `UserConstructionScript`)