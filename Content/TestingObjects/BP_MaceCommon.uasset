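; Common mace weapon for golems that damages an enemy golem when its MaceArm component overlaps one.
; The overlap, gated by CanAttack and HasAttacked, resolves the target from either a BP_Golem or a Part's associated golem.
; If team IDs differ, it prints a debug string, applies Damage with WeaponType and the owning golem as instigator, then sets HasAttacked to block further hits.
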(event `self.MaceArm.OnComponentBeginOverlap`
  (params (OverlappedComponent :type "PrimitiveComponent Object Reference") (OtherActor :type "Actor Object Reference") (OtherComp :type "PrimitiveComponent Object Reference") (OtherBodyIndex :type Integer) (bFromSweep :type Boolean) (SweepResult :type "HitResult Structure (by ref)"))
  (if (and (not (`self.HasAttacked`)) (`self.CanAttack`))
    (bind _asbp_golem (cast `/Game/Characters/Golem/BP_Golem` OtherActor)
      (:`then`
        (set `self.OtherGolem` _asbp_golem))
      (:`CastFailed`
        (bind _aspart (cast `Part` OtherActor))
        (bind _asbp_golem_2 (cast `/Game/Characters/Golem/BP_Golem` (`Part.associatedGolem` _aspart)))
        (set `self.OtherGolem` _asbp_golem_2)))
    (if (!= (`Golem.GenericTeamIDInt` (`self.OtherGolem`)) (`Golem.GenericTeamIDInt` (`self.associatedGolem`)))
      (`KismetSystemLibrary.PrintString` "MaceArmOverlap" true true (struct :`R` 1.0 :`B` 0.766562 :`A` 1.0))
      (`/Game/Characters/Golem/BP_Golem.ReceiveDamage` (`self.OtherGolem`) (`self.Damage`) "DT_Instant" (`self.WeaponType`) (`self.associatedGolem`))
      (set `self.HasAttacked` true))))

(fn `UserConstructionScript`)