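; BP_CannonCommon is a cannon part that shoots a physics projectile at a given target when used.
; UsePartImpl calls FireProjectile, which, once the cooldown has run out, spawns a bullet, records the cannon as its holder and offsets it along the Cube's forward vector.
; An impulse scaled by AddedForce launches the bullet toward the target, then the cooldown restarts.
; The cooldown countdown is not handled here, and ResetGolemTarget is an empty stub.
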(event `FireEventDispatcher_Event`
  (params (ShootTarget :type "Actor Object Reference") (GolemRef :type "/Game/Characters/Golem/BP_Golem Object Reference")))

(event `self.ReceiveTick`
  (params (DeltaSeconds :type "Float (single-precision)")))

(event `self.UsePartImpl`
  (params (target :type "Actor Object Reference"))
  (`self.FireProjectile` target))

(fn `FireProjectile`
  (params (Target :type "Actor Object Reference"))
  (locals (NewLocalVar :type "Actor Object Reference"))
  (if (<= (`self.CurrentCooldown`) 0.0)
    (bind _returnvalue (`|SpawnActorFromClass` "/Game/TestingObjects/BulletInGame.BulletInGame_C" (`KismetMathLibrary.MakeTransform` (`self.K2_GetActorLocation`) (`self.K2_GetActorRotation`)) "Undefined" "MultiplyWithRoot" null (`self.GetInstigator`)))
    (set `/Game/TestingObjects/BulletInGame.Holder` self _returnvalue)
    (`self.K2_SetActorLocation` _returnvalue (+ (`self.K2_GetActorLocation`) (* (`SceneComponent.GetForwardVector` (`self.Cube`)) (50.0 50.0 50.0))) false false)
    (`PrimitiveComponent.AddImpulse` (`/Game/TestingObjects/BulletInGame.Sphere` _returnvalue) (* (`KismetMathLibrary.Normal` (- (`self.K2_GetActorLocation` Target) (`SceneComponent.K2_GetComponentLocation` (`self.Cube`)))) (`self.AddedForce`)) "None" false)
    (set `self.CurrentCooldown` (`self.Cooldown`))))

(fn `ResetGolemTarget`)

(fn `UserConstructionScript`)