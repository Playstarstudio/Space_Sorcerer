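; BP_Laserbeam is a laser beam actor that stretches a cylinder mesh along its up vector to the first blocking object.
; Each tick, SetEndPoint box-traces on Visibility up to MaxRange and stores the result in HitInfo.
; The cylinder's Z scale follows the hit distance divided by 100, or uses MaxRange undivided when nothing blocks.
; ChangeColor runs on BeginPlay but is empty.
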(event `self.ReceiveBeginPlay`
  (`self.ChangeColor`))

(event `self.ReceiveTick`
  (params (DeltaSeconds :type "Float (single-precision)"))
  (`self.SetEndPoint`))

(fn `ChangeColor`)

(fn `SetEndPoint`
  (locals (MaxRange :type "Float (double-precision)" :default 500.0) (HitInfo :type "HitResult Structure"))
  (bind _returnvalue (`self.GetActorUpVector`))
  (bind _returnvalue_2 (+ (+ (`self.K2_GetActorLocation`) (0.0 0.0 0.0)) (* _returnvalue 2.0)))
  (bind _outhit (`KismetSystemLibrary.BoxTraceSingle` _returnvalue_2 (+ _returnvalue_2 (* _returnvalue (`local.MaxRange`))) (0.5 0.5 0.5) (struct) "TraceTypeQuery1"))
  (bind _output_get (set `local.HitInfo` _outhit))
  (bind (_bblockinghit _binitialoverlap _time _distance) (`GameplayStatics.BreakHitResult` _output_get))
  (`SceneComponent.SetWorldScale3D` (`self.Cylinder`) (`KismetMathLibrary.MakeVector` 0.5 0.5 (`KismetMathLibrary.SelectFloat` (/ (+ _distance 1.0) 100.0) (`local.MaxRange`) _bblockinghit))))

(fn `UserConstructionScript`)