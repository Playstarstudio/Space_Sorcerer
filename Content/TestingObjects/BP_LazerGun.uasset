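; BP_LazerGun is a test laser gun part that toggles a BP_Laserbeam on and off through UsePartImpl.
; ToggleLaser spawns a scaled beam attached to LaserArm's LaserPoint socket, or destroys it, while Tick updates its LaserTransform from that socket.
; UsePartImpl acts only while CurrentCooldown is above zero, and Tick's SelectFloat zeroes a positive laser timer instead of counting down.
; FireLaser is an empty stub.
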(event `self.ReceiveBeginPlay`)

(event `self.ReceiveTick`
  (params (DeltaSeconds :type "Float (single-precision)"))
  (set `self.CurrentLaserTimer` (`KismetMathLibrary.SelectFloat` (- (`self.CurrentLaserTimer`) DeltaSeconds) 0.0 (<= (- (`self.CurrentLaserTimer`) DeltaSeconds) 0.0)))
  (bind _laserbeam (`self.LaserBeam`)
    (:`then`
      (set `/Game/TestingObjects/BP_Laserbeam.LaserTransform` (`SceneComponent.GetSocketTransform` (`self.LaserArm`) "LaserPoint" "RTS_World") _laserbeam))
    (:`else`)))

(event `self.UsePartImpl`
  (params (target :type "Actor Object Reference"))
  (if (<= (`self.CurrentCooldown`) 0.0)
    _
    (elif (`self.LaserEnabled`)
      (if (<= (`self.CurrentLaserTimer`) 0.0)
        (`self.ToggleLaser`)
        (set `self.CurrentCooldown` (`self.Cooldown`)))
      (else
        (`self.ToggleLaser`)
        (set `self.CurrentLaserTimer` (`self.DurationOfLaser`))))))

(fn `FireLaser`
  (params (Time :type "Float (double-precision)")))

(fn `ToggleLaser`
  (bind _laserbeam (`self.LaserBeam`))
  (if (`self.LaserEnabled`)
    (`self.K2_DestroyActor` (`self.LaserBeam`))
    (set `self.LaserEnabled` false)
    (else
      (bind _returnvalue (`|SpawnActorFromClass` "/Game/TestingObjects/BP_Laserbeam.BP_Laserbeam_C" (`SceneComponent.GetSocketTransform` (`self.LaserArm`) "LaserPoint" "RTS_World") "Undefined" "MultiplyWithRoot" null (`self.GetInstigator`)))
      (bind _output_get (set `self.LaserBeam` _returnvalue))
      (`self.SetActorScale3D` _output_get (0.2 0.2 0.2))
      (`self.K2_SetActorRelativeRotation` _laserbeam (struct :`Pitch` 90.0) false false)
      (`self.K2_AttachToComponent` _laserbeam (`self.LaserArm`) "LaserPoint" "SnapToTarget" "KeepRelative" "KeepRelative" true)
      (set `self.LaserEnabled` true))))

(fn `UserConstructionScript`)