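; BP_Mace is a mace weapon that damages enemy golems on contact.
; When MaceArm begins overlapping a BP_Golem, it compares that golem's team ID to AssociatedGolem's and applies Damage if they differ, naming AssociatedGolem as instigator.
; Tick counts CurrentCooldown down to zero, but the overlap hit does not check or reset it.
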(event `self.MaceArm.OnComponentBeginOverlap`
  (params (OverlappedComponent :type "PrimitiveComponent Object Reference") (OtherActor :type "Actor Object Reference") (OtherComp :type "PrimitiveComponent Object Reference") (OtherBodyIndex :type Integer) (bFromSweep :type Boolean) (SweepResult :type "HitResult Structure (by ref)"))
  (bind _asbp_golem (cast `/Game/Characters/Golem/BP_Golem` OtherActor))
  (if (!= (`Golem.GenericTeamIDInt` _asbp_golem) (`Golem.GenericTeamIDInt` (`self.associatedGolem`)))
    (`/Game/Characters/Golem/BP_Golem.ReceiveDamage` _asbp_golem (`self.Damage`) "DT_Instant" 0 (`self.associatedGolem`))))

(event `self.ReceiveTick`
  (params (DeltaSeconds :type "Float (single-precision)"))
  (bind _current_cooldown (`self.Current Cooldown`))
  (set `self.Current Cooldown` (- _current_cooldown DeltaSeconds))
  (set `self.Current Cooldown` (`KismetMathLibrary.FMax` 0.0 _current_cooldown)))

(fn `UserConstructionScript`)